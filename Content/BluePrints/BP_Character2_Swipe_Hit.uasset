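; BP_Character2_Swipe_Hit is a short-lived hit volume, apparently for Character2's swipe attack, that damages pawns.
; When its Sphere component begins an overlap, it runs a sphere overlap query for pawns and applies fixed damage to each result, naming itself as damage causer.
; Tick destroys the actor once game time exceeds Delay, which acts as an absolute timestamp and is not set within this Blueprint's graphs.
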(event `self.Sphere.OnComponentBeginOverlap`
  (params (OverlappedComponent :type "PrimitiveComponent Object Reference") (OtherActor :type "Actor Object Reference") (OtherComp :type "PrimitiveComponent Object Reference") (OtherBodyIndex :type Integer) (bFromSweep :type Boolean) (SweepResult :type "HitResult Structure (by ref)"))
  (`KismetSystemLibrary.SphereOverlapActors` (0.0 0.0 0.0) 0.0 (`|MakeArray` "ObjectTypeQuery3" :!type "EObjectTypeQuery Enum"))
  (for _array_element _
    (`GameplayStatics.ApplyDamage` _array_element 7.0 null self)))

(event `self.ReceiveTick`
  (params (DeltaSeconds :type "Float (single-precision)"))
  (if (> (`GameplayStatics.GetTimeSeconds`) (`self.delay`))
    (`self.K2_DestroyActor`)))

(fn `UserConstructionScript`)